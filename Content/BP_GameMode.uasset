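; BP_GameMode is a game mode for a timed collection round, tracking points, combo, level and a game-over flag.
; StartGame, called on BeginPlay and Restart, resets state except Combo and starts a looping one-second Clock timer that ends the round at zero.
; ObjectCollected raises Combo and awards combo-scaled points.
; Its every-fifth-object check does nothing, ObjectCount never increments, and a combo bonus branch is disconnected.
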(event `Clock`
  (bind _output_get (set `self.Time` (- (`self.Time`) 1)))
  (if (== _output_get 0)
    (set `self.GameOver` true)
    (`KismetSystemLibrary.K2_ClearTimer` null "clock")))

(event `self.ReceiveBeginPlay`
  (`self.Start Game`))

(event `Restart`
  (`self.Start Game`))

(fn `Object Collected`
  (bind _output_get (set `self.Combo` (+ (`self.Combo`) 1)))
  (set `self.Points` (+ (`self.Points`) (* _output_get 10) 0))
  (bind _output_get_2 (set `self.ObjectCount` (+ (`self.ObjectCount`) 0)))
  (if (== (mod _output_get_2 5) 0)
    _))

(fn `UserConstructionScript`)