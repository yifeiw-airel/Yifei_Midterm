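; BP_Object is a collectible that keeps jumping to random spots within a fixed area at a constant height.
; InitialObject teleports it and re-arms its own timer, with a delay that shrinks as the BP_GM game mode's player level rises.
; When the player character overlaps it before game over, it notifies the game mode, destroys itself and spawns an actor at its transform.
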(event `self.ReceiveBeginPlay`
  (bind _asbp_gm (cast `/Game/BP_GM` (`GameplayStatics.GetGameMode`)))
  (set `self.Game mode` _asbp_gm)
  (`self.InitialObject`))

(event `self.ReceiveActorBeginOverlap`
  (params (OtherActor :type "Actor Object Reference"))
  (if (and (== OtherActor (`GameplayStatics.GetPlayerCharacter` 0)) (not (`/Game/BP_GM.Game Over` (`self.Game mode`))))
    (`/Game/BP_GM.Object Collected` (`self.Game mode`))
    (`self.K2_DestroyActor`)
    (`|SpawnActorFromClass` "/Script/Engine.Actor" (`self.GetTransform`) "Undefined" "MultiplyWithRoot" null null)))

(fn `InitialObject`
  (`self.K2_TeleportTo` (`KismetMathLibrary.MakeVector` (`KismetMathLibrary.RandomFloatInRange` 100.0 1000.0) (`KismetMathLibrary.RandomFloatInRange` 300.0 1400.0) 130.0))
  (`KismetSystemLibrary.K2_SetTimer` null "InitialObject" (`KismetMathLibrary.Conv_IntToDouble` (- 6 (`/Game/BP_GM.PlayerLevel` (`self.Game mode`))))))

(fn `UserConstructionScript`)