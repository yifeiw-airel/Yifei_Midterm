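; BP_GM holds the rules and state for a timed collection game: countdown, score, combo, player level and game-over flag.
; StartGame resets state on BeginPlay or restart and starts a looping one-second Clock timer that ends the game at zero.
; ObjectCollected raises the level every fifth pickup up to a cap, and builds combo bonuses while enough time remains.
; A disconnected branch holds an unused time-bonus round mechanic.
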(event `Clock`
  (bind _output_get (set `self.Time` (- (`self.Time`) 1)))
  (if (== _output_get 0)
    (set `self.Game Over` true)
    (`KismetSystemLibrary.K2_ClearTimer` null "clock")))

(event `self.ReceiveBeginPlay`
  (`self.Start Game`))

(event `RestartGame_Event`
  (`self.Start Game`))

(fn `Object Collected`
  (`|ExecutionSequence`
    (:`then_0`
      (bind _output_get (set `self.ObjectCount` (+ (`self.ObjectCount`) 1)))
      (if (== (mod _output_get 5) 0)
        (set `self.PlayerLevel` (`KismetMathLibrary.Min` (+ (`self.PlayerLevel`) 1) 5))))
    (:`then_1`
      (if (>= (`self.Time`) 15)
        (set `self.Combo` (+ (`self.Combo`) 1))
        (set `self.Points` (+ (`self.Points`) (* (`self.Combo`) 10) 0))
        (if (>= (`self.Combo`) 3)
          (set `self.Points` (+ (`self.Points`) 100))
          (set `self.Combo` 0)
          (set `self.Points` (+ (`self.Points`) (* (`self.Combo`) 10) 0)))
        (else
          (bind _output_get_2 (set `self.Combo` 1))
          (set `self.Points` (+ (`self.Points`) (* _output_get_2 10) 0)))))))

(fn `UserConstructionScript`)